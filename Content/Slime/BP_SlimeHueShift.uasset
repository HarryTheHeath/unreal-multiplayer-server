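; Slime hazard actor that slows overlapping characters and repeatedly changes their health by a randomly signed amount.
; On BeginPlay it randomizes its position, scale, material hue and inversion parameters, picks the health effect's sign, and loops a vertical bobbing Timeline.
; Overlap lowers walk speed to crouched speed and starts a DoOnce-gated delay loop applying GE_ReduceHealth through GAS with a SetByCaller magnitude.
; End overlap stops the loop and sets a fixed walk speed.
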(event OnComponentBeginOverlap(Sphere)
  (params (OverlappedComponent :type Primitive%20Component%20Object%20Reference) (OtherActor :type Actor%20Object%20Reference) (OtherComp :type Primitive%20Component%20Object%20Reference) (OtherBodyIndex :type Integer) (bFromSweep :type Boolean) (SweepResult :type Hit%20Result%20Structure%20%28by%20ref%29))
  (bind _returnvalue (Actor|GetComponentbyClass OtherActor "/Script/Engine.CharacterMovementComponent"))
  (bind _asbp_third_person_character (Utilities|Casting|CastToBP_ThirdPersonCharacter OtherActor))
  (bind _returnvalue_2 (Actor|GetComponentbyClass _asbp_third_person_character "/Script/UnrealGP.GPAbilitySystemBase"))
  (if (Utilities|IsValid _returnvalue)
    (Utilities|FlowControl|DoOnce false
      (:Completed
        (Variables|/Script/Engine.CharacterMovementComponent|SetMaxWalkSpeed _returnvalue (Variables|/Script/Engine.CharacterMovementComponent|GetMaxWalkSpeedCrouched _returnvalue))
        (bind _output_get (Variables|Default|SetOverlapping true))
        (if _output_get :!label _label
          (bind _returnvalue_3 (Ability|GameplayEffect|AssignTagSetbyCallerMagnitude (GameplayEffects|MakeOutgoingSpec :self _returnvalue_2 :GameplayEffectClass "/Game/ThirdPerson/Blueprints/Effects/GE_ReduceHealth.GE_ReduceHealth_C") "(TagName=\"SetByCaller.Magnitude\")" (Variables|Default|GetDamage)))
          (GameplayEffects|ApplyGameplayEffectSpecToSelf _returnvalue_2 _returnvalue_3)
          (Utilities|FlowControl|Delay 0.2)
          (goto _label))))))

(event OnComponentEndOverlap(Sphere)
  (params (OverlappedComponent :type Primitive%20Component%20Object%20Reference) (OtherActor :type Actor%20Object%20Reference) (OtherComp :type Primitive%20Component%20Object%20Reference) (OtherBodyIndex :type Integer))
  (bind _returnvalue (Actor|GetComponentbyClass OtherActor "/Script/Engine.CharacterMovementComponent"))
  (if (Utilities|IsValid _returnvalue)
    (Variables|Default|SetOverlapping false)
    (Variables|/Script/Engine.CharacterMovementComponent|SetMaxWalkSpeed _returnvalue 5e+02)
    (Utilities|FlowControl|DoOnce false) ; enters at Reset
  ))

(event Custom|Update%20locations
  (Transformation|SetActorTransform (Math|Transform|MakeTransform (Math|Vector|MakeVector (Math|Conversions|ToFloat(Integer) (+ (Math|Random|RandomInteger 4150) 450)) (Math|Conversions|ToFloat(Integer) (+ (Math|Random|RandomInteger 4600) 450)) 0.0) "0, 0, 0" (Math|Conversions|ToVector(Float) (Math|Random|RandomFloatinRange 0.5 2.0))))
  (Rendering|Material|SetScalarParameterValueonMaterials (Variables|Default|GetSlimeSphere) "HueShift" (Math|Random|RandomFloat))
  (Rendering|Material|SetScalarParameterValueonMaterials (Variables|Default|GetSlimeSphere) "NoiseInverse" (Math|Conversions|ToFloat(Boolean) (Math|Random|RandomBool)))
  (Rendering|Material|SetScalarParameterValueonMaterials (Variables|Default|GetSlimeSphere) "Inverse" (Math|Conversions|ToFloat(Boolean) (Math|Random|RandomBool)))
  (bind _newtrack_0 (Timeline|Timeline_0 Play)
    (:Update
      (Transformation|SetRelativeLocation (Variables|Default|GetSlimeSphere) (Math|Vector|MakeVector 0.0 0.0 _newtrack_0) false false))
    (:Finished
      (Timeline|Timeline_0 PlayFromStart))))

(event Custom|SetHealthEffect
  (Variables|Default|SetDamage (Math|Float|SelectFloat 2.0 -2.0 (Math|Random|RandomBool))))

(event EventBeginPlay
  (CallFunction|UpdateLocations)
  (CallFunction|SetHealthEffect))

(fn ConstructionScript)

(fn OnRepDamage)