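; BP_SlimeRave is a slime sphere actor that bobs and flickers through random material looks.
; A timeline starts on BeginPlay, drives the sphere's relative Z and replays itself on finish.
; Its update also runs through a short Delay that throttles randomizing hue shift and two inversion toggles via material scalar parameters.
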(event EventBeginPlay
  (bind _newtrack_0 (Timeline|Timeline_0 Play)
    (:Update
      (Transformation|SetRelativeLocation (Variables|Default|GetSlimeSphere) (Math|Vector|MakeVector 0.0 0.0 _newtrack_0) false false)
      (Utilities|FlowControl|Delay 0.125)
      (Rendering|Material|SetScalarParameterValueonMaterials (Variables|Default|GetSlimeSphere) "HueShift" (Math|Random|RandomFloat))
      (Rendering|Material|SetScalarParameterValueonMaterials (Variables|Default|GetSlimeSphere) "Inverse" (Math|Conversions|ToFloat(Boolean) (Math|Random|RandomBool)))
      (Rendering|Material|SetScalarParameterValueonMaterials (Variables|Default|GetSlimeSphere) "NoiseInverse" (Math|Conversions|ToFloat(Boolean) (Math|Random|RandomBool))))
    (:Finished
      (Timeline|Timeline_0 PlayFromStart))))

(fn ConstructionScript)